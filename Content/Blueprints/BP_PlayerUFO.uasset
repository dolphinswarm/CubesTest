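; Player-controlled UFO pawn that flies on three axes, drops physical blocks and fires a laser that shoves physics objects.
; A downward trace each tick sets the height of a crosshair plane on the surface below.
; Dropped blocks spawn beneath the UFO with the chosen class, size and material, with mass overridden by material type.
; The laser traces from the mouse cursor, applying an unnormalized impulse away from the UFO that grows with distance.
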(event EventTick
  (params (DeltaSeconds :type Float%20%28single-precision%29))
  (bind _returnvalue (Transformation|GetActorLocation))
  (bind _plane (Variables|Default|GetPlane))
  (bind _returnvalue_2 (Transformation|GetWorldLocation _plane))
  (bind (_x _y) (Math|Vector|BreakVector _returnvalue_2))
  ;[0.1116 1 0] Raycasting to set the Z-Height of the Crosshair
  (bind _outhit (Collision|LineTraceForObjects _returnvalue (+ _returnvalue "0, 0,-5000.000000") (Utilities|Array|MakeArray "ObjectTypeQuery4" "ObjectTypeQuery1") false 0 "None"))
  (Transformation|SetWorldLocation _plane (Math|Vector|MakeVector _x _y (+ (.Z (Math|Vector|BreakVector (.ImpactPoint (Collision|BreakHitResult _outhit)))) 1.0)) false false))

(event Input|ActionEvents|InputActionDropBlock
  (params (Key :type Key%20Structure :default "None"))
  (bind _blocksize (Variables|Default|GetBlockSize))
  ;[0.8564 1 0.7459] Spawn Block
  (:Pressed
    (bind _returnvalue (Game|SpawnActorfromClass (Variables|Default|GetBlockToSpawn) (Math|Conversions|ToTransform(Vector) (+ (Transformation|GetActorLocation) (Math|Vector|MakeVector 0.0 0.0 (* (Variables|Default|GetBlockSize) -125.0)))) "Undefined" 0 0))
    (Transformation|SetActorScale3D _returnvalue (Math|Vector|MakeVector _blocksize _blocksize _blocksize))
    (bind _asstatic_mesh_actor (Utilities|Casting|CastToStaticMeshActor _returnvalue))
    (Rendering|Material|SetMaterial (Variables|/Script/Engine.StaticMeshActor|GetStaticMeshComponent _asstatic_mesh_actor) 0 (Variables|Default|GetMaterialToUse))
    (Class|PrimitiveComponent|SetMassOverrideinKg (Variables|/Script/Engine.StaticMeshActor|GetStaticMeshComponent _asstatic_mesh_actor) "None" (* (Utilities|Select :Index (Variables|Default|GetSelectedMaterial) :NewEnumerator1 1.0 :NewEnumerator2 1.0 :NewEnumerator3 1e+01 :NewEnumerator4 1e+01 :NewEnumerator6 5.0 :NewEnumerator7 0.5) 1e+02) true)))

(event Input|ActionEvents|InputActionFireLaser
  (params (Key :type Key%20Structure :default "None"))
  (bind _returnvalue (Game|GetPlayerController 0))
  (bind (_worldlocation _worlddirection) (Game|Player|ConvertMouseLocationToWorldSpace _returnvalue))
  ;[1 0.2215 0.8664] Fire Laser
  (:Pressed
    (bind (_outhit _returnvalue_2) (Collision|LineTraceForObjects _worldlocation (+ _worldlocation (* _worlddirection 5e+03)) (Utilities|Array|MakeArray "ObjectTypeQuery4") false 0 "None" false))
    (if _returnvalue_2
      (Physics|AddImpulse (.HitComponent (Collision|BreakHitResult _outhit)) (* (- (Transformation|GetActorLocation (.HitActor (Collision|BreakHitResult _outhit))) (Transformation|GetActorLocation)) 1e+03) "None" false))))

(event Input|AxisEvents|InputAxisForward
  (params (AxisValue :type Float%20%28single-precision%29))
  ;[0 0.5532 1] UFO Movement
  (Pawn|Input|AddMovementInput (Transformation|GetActorForwardVector) (* AxisValue 1e+03) false))

(event Input|AxisEvents|InputAxisHorizontal
  (params (AxisValue :type Float%20%28single-precision%29))
  ;[0 0.5532 1] UFO Movement
  (Pawn|Input|AddMovementInput (Transformation|GetActorRightVector) (* AxisValue 1e+03) false))

(event Input|AxisEvents|InputAxisVertical
  (params (AxisValue :type Float%20%28single-precision%29))
  ;[0 0.5532 1] UFO Movement
  (Pawn|Input|AddMovementInput (Transformation|GetActorUpVector) (* AxisValue 1e+03) false))

(fn ConstructionScript)