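; NewPlayerController lets the player launch cubes with the Space Bar.
; Each press spawns a Cube_Blueprint at the player pawn's transform, then applies a strong mass-dependent impulse to its static mesh along the control rotation's forward vector.
; A step to align the cube with the control rotation is left unconnected, so it never runs.
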(event EventBeginPlay)

(event EventTick
  (params (DeltaSeconds :type Float%20%28single-precision%29)))

(event Input|KeyboardEvents|SpaceBar
  (params (Key :type Key%20Structure :default "None"))
  (bind _returnvalue (Game|Player|GetPlayerPawn 0))
  (:Pressed
    (bind _returnvalue_2 (Game|SpawnActorfromClass "/Game/Cube_Blueprint.Cube_Blueprint_C" (Transformation|GetActorTransform _returnvalue) "Undefined" 0 0))
    (Physics|AddImpulse (Variables|/Script/Engine.StaticMeshActor|GetStaticMeshComponent _returnvalue_2) (* (Math|Vector|GetForwardVector (Pawn|GetControlRotation _returnvalue :!class /Script/Engine.Pawn)) 3e+04) "None" false)))

(fn ConstructionScript)